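; Player controller for the Warlocks game that keeps the spell UI in sync and highlights the character under the cursor.
; When granted abilities change, it finds the player UI widget and refreshes its spell display.
; Every tick it clears the outline on all Warlocks characters, then enables it on the one hit by a cursor pawn trace.
; Leaving a session in progress opens the main map.
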(event Custom|LeaveSessionInProgress
  (Game|OpenLevel(byObjectReference) "/Game/Warlocks/Maps/MainMap.MainMap"))

(event Custom|OnGrantedAbilitiesDelegate_Event
  (bind _foundwidgets (Widget|GetAllWidgetsOfClass "/Game/Warlocks/Blueprints/Widgets/Game/WBP_PlayerUI.WBP_PlayerUI_C" true))
  (if (!= (Utilities|Array|Length _foundwidgets) 0)
    (Default|UpdateSpellUI (Utilities|Array|Get(acopy) _foundwidgets))))

(event EventTick
  (params (DeltaSeconds :type Float%20%28single-precision%29))
  (bind _outactors (Actor|GetAllActorsOfClass "/Game/Warlocks/Blueprints/Game/BP_WarlocksCharacter_1.BP_WarlocksCharacter_1_C"))
  (for _array_element _outactors
    (Default|SetIsOutlineVisible _array_element false))
  (bind _asbp_warlocks_character_1 (Utilities|Casting|CastToBP_WarlocksCharacter_1 (.HitActor (Collision|BreakHitResult (.HitResult (Class|PlayerController|GetHitResultUnderCursorforObjects (Utilities|Array|MakeArray "ObjectTypeQuery3") true))))))
  (Default|SetIsOutlineVisible _asbp_warlocks_character_1 true))

(event EventBeginPlay
  (EventDispatchers|BindEventtoOnGrantedAbilitiesDelegate (delegate Custom|OnGrantedAbilitiesDelegate_Event)))

(fn ConstructionScript)