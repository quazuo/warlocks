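; BP_WarlocksGameMode is the game mode for Warlocks that caps how many players join a match.
; On PostLogin it casts the new controller to BP_WarlocksPlayerController and compares the PlayerList size to the "playercount" value parsed from the options string.
; Players within the limit are added to PlayerList; others are told to leave the session in progress.
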(event EventBeginPlay)

(event EventTick
  (params (DeltaSeconds :type Float%20%28single-precision%29)))

(event EventPostLogin
  (params (NewPlayer :type Player%20Controller%20Object%20Reference))
  (bind _asbp_warlocks_player_controller (Utilities|Casting|CastToBP_WarlocksPlayerController NewPlayer))
  (if (< (Utilities|Array|Length (Variables|Default|GetPlayerList)) (Math|Conversions|ToInteger(Byte) (.OutValue (Class|KismetSystemLibrary|ParseParamValue (Variables|Default|GetOptionsString) "playercount"))))
    (Utilities|Array|Add (Variables|Default|GetPlayerList) _asbp_warlocks_player_controller)
    (else
      (Default|LeaveSessioninProgress _asbp_warlocks_player_controller))))

(fn ConstructionScript)