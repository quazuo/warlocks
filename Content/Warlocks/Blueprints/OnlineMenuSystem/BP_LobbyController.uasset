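; Lobby controller for the online menu system that shows each player a lobby screen and tracks their ready state.
; On BeginPlay it creates either the host or client lobby widget, based on network authority.
; UpdatePlayerList stores the connected players and forwards them to that widget.
; SetReadyStatus flips the ready flag in PlayerInfo, then has BP_LobbyGameMode refresh the player lists.
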(event Custom|CreateMenu
  (Networking|SwitchHasAuthority
    (:Authority
      (bind _returnvalue (UserInterface|CreateWidget "/Game/Warlocks/Blueprints/Widgets/MainMenu/WBP_LobbyHost.WBP_LobbyHost_C"))
      (bind _output_get (Variables|Default|SetLobbyWidget _returnvalue))
      (UserInterface|Viewport|AddtoViewport _output_get 0)
      (Development|PrintString "cr server"))
    (:Remote
      (bind _returnvalue_2 (UserInterface|CreateWidget "/Game/Warlocks/Blueprints/Widgets/MainMenu/WBP_LobbyClient.WBP_LobbyClient_C"))
      (bind _output_get_2 (Variables|Default|SetLobbyWidget _returnvalue_2))
      (UserInterface|Viewport|AddtoViewport _output_get_2 0)
      (Development|PrintString "cr client"))))

(event Custom|UpdatePlayerList
  (params (Connected%20Players :type Array%20of%20BP%20Player%20Info%20Structure%20Structures))
  (bind _lobbywidget (Variables|Default|GetLobbyWidget))
  (Variables|Default|SetConnected%20Players Connected%20Players)
  (Networking|SwitchHasAuthority
    (:Authority
      (bind _aswbp_lobby_host (Utilities|Casting|CastToWBP_LobbyHost _lobbywidget))
      (Default|UpdatePlayerList _aswbp_lobby_host (Variables|Default|GetConnected%20Players))
      (Development|PrintString "siema server"))
    (:Remote
      (bind _aswbp_lobby_client (Utilities|Casting|CastToWBP_LobbyClient _lobbywidget))
      (Default|UpdatePlayerList _aswbp_lobby_client (Variables|Default|GetConnected%20Players))
      (Development|PrintString "siema client"))))

(event Custom|SetReadyStatus
  (bind _player_info (Variables|Default|GetPlayer%20Info))
  (Utilities|Struct|SetmembersinBP_PlayerInfoStructure _player_info (not (.bIsReady (Utilities|Struct|BreakBP_PlayerInfoStructure _player_info))))
  (bind _asbp_lobby_game_mode (Utilities|Casting|CastToBP_LobbyGameMode (Game|GetGameMode)))
  (Default|UpdatePlayerLists _asbp_lobby_game_mode))

(event EventBeginPlay
  (CallFunction|CreateMenu))

(event EventTick
  (params (DeltaSeconds :type Float%20%28single-precision%29)))

(fn ConstructionScript)