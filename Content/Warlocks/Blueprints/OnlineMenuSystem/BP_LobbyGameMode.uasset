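; Lobby game mode for the online menu system that tracks connected players and shares their info with every lobby controller.
; On login, it stores the BP_LobbyController and its info, then broadcasts the list after a short delay.
; UpdatePlayerLists rebuilds the info list from all controllers before running that same broadcast loop.
; Both paths mark the local controller as a ready player named HOST.
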(event Custom|UpdatePlayerLists
  (Utilities|Array|Clear (Variables|Default|GetConnected%20Player%20Info))
  (for _array_element (Variables|Default|GetConnected%20Players)
    (if (Pawn|IsLocalController _array_element)
      (Variables|/Game/Warlocks/Blueprints/OnlineMenuSystem/BP_LobbyController.BP_LobbyController_C|SetPlayer%20Info _array_element (Utilities|Struct|MakeBP_PlayerInfoStructure "HOST" true 0)))
    (Utilities|Array|Add (Variables|Default|GetConnected%20Player%20Info) (Variables|/Game/Warlocks/Blueprints/OnlineMenuSystem/BP_LobbyController.BP_LobbyController_C|GetPlayer%20Info _array_element)))
  (for _array_element_2 (Variables|Default|GetConnected%20Players)
    (Default|UpdatePlayerList _array_element_2 (Variables|Default|GetConnected%20Player%20Info))))

(event EventBeginPlay)

(event EventTick
  (params (DeltaSeconds :type Float%20%28single-precision%29)))

(event EventPostLogin
  (params (NewPlayer :type Player%20Controller%20Object%20Reference))
  (bind _asbp_lobby_controller (Utilities|Casting|CastToBP_LobbyController NewPlayer))
  (if (Pawn|IsLocalController _asbp_lobby_controller)
    (Variables|/Game/Warlocks/Blueprints/OnlineMenuSystem/BP_LobbyController.BP_LobbyController_C|SetPlayer%20Info _asbp_lobby_controller (Utilities|Struct|MakeBP_PlayerInfoStructure "HOST" true 0)))
  (Utilities|Array|Add (Variables|Default|GetConnected%20Players) _asbp_lobby_controller)
  (Utilities|Array|Add (Variables|Default|GetConnected%20Player%20Info) (Variables|/Game/Warlocks/Blueprints/OnlineMenuSystem/BP_LobbyController.BP_LobbyController_C|GetPlayer%20Info _asbp_lobby_controller))
  (Utilities|FlowControl|Delay 0.5)
  (for _array_element (Variables|Default|GetConnected%20Players)
    (Default|UpdatePlayerList _array_element (Variables|Default|GetConnected%20Player%20Info))))

(fn ConstructionScript)